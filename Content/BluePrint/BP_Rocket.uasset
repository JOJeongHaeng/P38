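; BP_Rocket is a rocket actor that explodes and deals damage when it overlaps another actor.
; Overlaps with actors tagged Player are ignored; any other overlap spawns explosion effects and sound, applies fixed damage credited to the instigator's controller, then destroys the rocket.
; A short life span set on BeginPlay removes rockets that hit nothing, without an explosion.
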(event `self.ReceiveBeginPlay`
  (`self.SetLifeSpan` 3.0))

(event `self.ReceiveActorBeginOverlap`
  (params (OtherActor :type "Actor Object Reference"))
  (bind _returnvalue (`self.K2_GetActorLocation`))
  (if (not (`self.ActorHasTag` OtherActor "Player"))
    (`GameplayStatics.SpawnEmitterAtLocation` "/Game/StarterContent/Particles/P_Explosion.P_Explosion" _returnvalue)
    (`GameplayStatics.SpawnSoundAtLocation` "/Game/StarterContent/Audio/Explosion_Cue.Explosion_Cue" _returnvalue (struct) 1.0 1.0 0.0 null null)
    (`GameplayStatics.ApplyDamage` OtherActor 100.0 (`self.GetInstigatorController`) self)
    (`self.K2_DestroyActor`)))

(fn `UserConstructionScript`)